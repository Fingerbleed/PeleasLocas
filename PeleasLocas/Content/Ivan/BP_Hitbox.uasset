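; BP_Hitbox is a short-lived attack hitbox that destroys itself after HitboxDuration.
; Its construction script sizes the Box in X and Z with fixed Y depth and offsets it by PosX and PosZ.
; On overlap with anything but another hitbox or the Player, it builds the Player's meter by DamageToDeal unless IsMetered, then prints the meter.
; It applies no damage to the overlapped actor.
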(event `self.ReceiveBeginPlay`
  (`KismetSystemLibrary.Delay` (`self.hitboxDuration`))
  (`self.K2_DestroyActor`))

(event `self.Box.OnComponentBeginOverlap`
  (params (OverlappedComponent :type "PrimitiveComponent Object Reference") (OtherActor :type "Actor Object Reference") (OtherComp :type "PrimitiveComponent Object Reference") (OtherBodyIndex :type Integer) (bFromSweep :type Boolean) (SweepResult :type "HitResult Structure (by ref)"))
  (bind _player (`self.player`))
  (if (or (== (`GameplayStatics.GetObjectClass` OtherActor) "BP_Hitbox_C") (== OtherActor (`self.player`)))
    _
    (elif (`self.isMetered`)
      (`KismetSystemLibrary.PrintString` (`KismetStringLibrary.Concat_StrStr` "Meter: " (`KismetStringLibrary.Conv_IntToString` (`/Game/Ivan/BP_ThirdPersonCharacter1.meter` _player))))
      (else
        (`/Game/Ivan/BP_ThirdPersonCharacter1.MeterBuild` _player (`self.damageToDeal`))
        (`KismetSystemLibrary.PrintString` (`KismetStringLibrary.Concat_StrStr` "Meter: " (`KismetStringLibrary.Conv_IntToString` (`/Game/Ivan/BP_ThirdPersonCharacter1.meter` _player))))))))

(fn `UserConstructionScript`
  (bind _box (`self.Box`))
  (`BoxComponent.SetBoxExtent` _box (`KismetMathLibrary.MakeVector` (`self.sizeX`) 16.0 (`self.sizeZ`)) true)
  (`SceneComponent.K2_SetRelativeLocation` _box (+ (`SceneComponent.RelativeLocation` _box) (`KismetMathLibrary.MakeVector` (`self.posX+-`) 0.0 (`self.posZ+-`))) false true))