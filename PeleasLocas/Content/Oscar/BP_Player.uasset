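; BP_Player is a player pawn Blueprint with basic movement and a health value.
; On BeginPlay it adds the IMC_Player Enhanced Input mapping context and initializes current health to the maximum.
; IA_FMove drives movement along the fixed world X axis.
; The 0 key acts as a debug damage input that lowers health and prints a death message once it reaches zero.
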(event `self.ReceiveBeginPlay`
  (bind _asplayer_controller (cast `PlayerController` (`self.GetController`)))
  (bind _returnvalue (pcsubsystem `EnhancedInputLocalPlayerSubsystem` _asplayer_controller))
  (`/Engine/EditorBlueprintResources/StandardMacros.IsValid` _returnvalue
    (:`Is Valid`
      (`EnhancedInputSubsystemInterface.AddMappingContext` _returnvalue "/Game/Oscar/IMC_Player.IMC_Player" 0 (struct))
      (set `self.MaxHealth` 100.0)
      (set `self.CurrentHealth` (`self.MaxHealth`)))))

(event `EnhancedInput|/Game/Oscar/IA_FMove`
  (params (ActionValue :type "Float (double-precision)") (ElapsedSeconds :type "Float (double-precision)") (TriggeredSeconds :type "Float (double-precision)") (InputAction :type "InputAction Object Reference" :default "/Game/Oscar/IA_FMove.IA_FMove"))
  (:`Triggered`
    (`self.AddMovementInput` (1.0 0.0 0.0) ActionValue)))

(event `Key|Zero`
  (params (Key :type "Key Structure"))
  (:`Pressed`
    (set `self.CurrentHealth` (- (`self.CurrentHealth`) 10.0))
    (if (<= (`self.CurrentHealth`) 0.0)
      (`KismetSystemLibrary.PrintText` "morite loco"))))

(fn `UserConstructionScript`)