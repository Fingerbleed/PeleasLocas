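; Game manager for a two-player battle that creates the battle and begin/end widgets and runs round flow.
; BeginPlay passes GameInstance character picks to the UI and to stubbed player creation.
; Tick updates health/meter, increments a character's UI stock at zero health, then either restarts the countdown or ends the game at two stocks.
; Spawning, stat reads and resets are placeholders: players stay None and values are zero.
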(event `self.ReceiveBeginPlay`
  (bind _returnvalue (`|CreateWidget` "/Game/_Kai/WBP_BattleUI.WBP_BattleUI_C"))
  (bind _output_get (set `self.BattleUI` _returnvalue))
  (bind _aswbp_battle_ui (cast `/Game/_Kai/WBP_BattleUI` _output_get))
  (bind _asbp_game_instance (cast `/Game/_Kai/BP_GameInstance` (`GameplayStatics.GetGameInstance`)))
  (set `/Game/_Kai/WBP_BattleUI.Character1Image` (`/Game/_Kai/BP_GameInstance.Player1Image` _asbp_game_instance) _aswbp_battle_ui)
  (set `/Game/_Kai/WBP_BattleUI.Character2Image` (`/Game/_Kai/BP_GameInstance.Player2Image` _asbp_game_instance) _aswbp_battle_ui)
  (`self.CreatePlayer` 0 (`/Game/_Kai/BP_GameInstance.Player1Index` _asbp_game_instance))
  (`self.CreatePlayer` 1 (`/Game/_Kai/BP_GameInstance.Player2Index` _asbp_game_instance))
  (bind _returnvalue_2 (`|CreateWidget` "/Game/_Kai/WBP_BeginEnd.WBP_BeginEnd_C"))
  (set `self.BeginEndWidget` _returnvalue_2))

(event `CreatePlayer`
  (params (`Player Index` :type Integer) (`Character Index` :type Integer))
  ;[1 1 1] DEBE MODIFICARSE PARA IMPLEMENTAR JUGADORES
  (switch `int` `Character Index`
    (:`Default`
      (`KismetSystemLibrary.PrintString` "Spawn Character 1" :!label _label))
    (:`0`
      (goto _label))
    (:`1`
      (`KismetSystemLibrary.PrintString` "Spawn Character 2")))
  (`KismetSystemLibrary.PrintString` (`KismetTextLibrary.Conv_TextToString` (`|FormatText` "Set Player {0} Position, Controller, Etc" `Player Index`)))
  (switch `int` `Player Index`
    (:`0`
      (set `self.Player1` null))
    (:`1`
      (set `self.Player2` null))))

(event `self.ReceiveTick`
  (params (DeltaSeconds :type "Float (single-precision)"))
  (if (not (`GameplayStatics.IsGamePaused`))
    (`/Engine/EditorBlueprintResources/StandardMacros.IsValid` (`self.Player1`)
      (:`Is Valid`
        (`/Engine/EditorBlueprintResources/StandardMacros.IsValid` (`self.Player2`)
          (:`Is Valid`
            (`self.SetCharacterValues` (`self.Player1`))
            (`self.SetCharacterValues` (`self.Player2`) 1)
            (bind _endround (`self.Check For Stock`))
            (if _endround
              (`KismetSystemLibrary.PrintString` "ResetCharacters") ; MODIFICAR PARA IMPLEMENTAR JUGADORES
              (`self.EndRound`))))))))

(event `SetCharacterValues`
  (params (Character :type "Actor Object Reference") (PlayerIndex :type Integer))
  ;[1 1 1] DEBE MODIFICARSE PARA AGREGAR JUGADORES
  (`KismetSystemLibrary.PrintString` "CastToCharacter")
  (`KismetSystemLibrary.PrintString` "GetHealth&Meter")
  (bind _aswbp_battle_ui (cast `/Game/_Kai/WBP_BattleUI` (`self.BattleUI`)))
  (switch `int` PlayerIndex
    (:`0`
      (`/Game/_Kai/WBP_BattleUI.SetCharacter1Health&Meter` _aswbp_battle_ui 0.0 0.0 0.0))
    (:`1`
      (`/Game/_Kai/WBP_BattleUI.SetCharacter2Health&meter` _aswbp_battle_ui 0.0 0.0 0.0))))

(event `EndRound`
  (bind _aswbp_battle_ui (cast `/Game/_Kai/WBP_BattleUI` (`self.BattleUI`)))
  (bind _aswbp_begin_end (cast `/Game/_Kai/WBP_BeginEnd` (`self.BeginEndWidget`)))
  (if (== 2 (`/Game/_Kai/WBP_BattleUI.Character1Stocks` _aswbp_battle_ui))
    (set `self.WinIndex` 1)
    (set `/Game/_Kai/WBP_BeginEnd.Index` -2 _aswbp_begin_end :!label _label_2)
    (`/Game/_Kai/WBP_BeginEnd.EndGame` _aswbp_begin_end (`self.WinIndex`))
    (elif (== 2 (`/Game/_Kai/WBP_BattleUI.Character2Stocks` _aswbp_battle_ui))
      (set `self.WinIndex` 2)
      (goto _label_2)
      (else
        (`/Game/_Kai/WBP_BeginEnd.BeginCountdown` _aswbp_begin_end)))))

(fn `Check For Stock`
  (returns (EndRound :type Boolean))
  (set `self.HasStock` false)
  (bind _aswbp_battle_ui (cast `/Game/_Kai/WBP_BattleUI` (`self.BattleUI`)))
  (if (== 0.0 (`/Game/_Kai/WBP_BattleUI.Character1Health` _aswbp_battle_ui))
    (`/Engine/EditorBlueprintResources/StandardMacros.IncrementInt` (`/Game/_Kai/WBP_BattleUI.Character1Stocks` _aswbp_battle_ui)
      (:`  `
        (set `self.HasStock` true))))
  (if (== 0.0 (`/Game/_Kai/WBP_BattleUI.Character2Health` _aswbp_battle_ui))
    (`/Engine/EditorBlueprintResources/StandardMacros.IncrementInt` (`/Game/_Kai/WBP_BattleUI.Character2Stocks` _aswbp_battle_ui)
      (:`  `
        _))
    (elif (`self.HasStock`)
      _
      (else
        (return false))))
  (return true))

(fn `UserConstructionScript`)